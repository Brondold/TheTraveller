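; Actor component for a toggleable lock-on targeting system on a Character.
; While a target is set, Tick stops movement-driven rotation, aims control rotation at the target and eases the spring arm offset.
; FindTarget sphere-traces pawns along camera forward but only prints the hit count; its result logic is disconnected.
; Dot-product target scoring looks unfinished, and the FaceTargetDirection yaw helper is not called here.
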(event Custom|Event_ToggleTargeting
  (Variables|Default|GetCurrentTarget
    (:then
      (CallFunction|EventUntarget))
    (:else
      (CallFunction|EventTryFindTarget))))

(event Custom|Event_TryFindTarget
  (bind (_return_value _found_target) (CallFunction|FindTarget))
  (if _return_value
    (Variables|Default|SetCurrentTarget _found_target)))

(event Custom|Event_Untarget
  (Variables|Default|SetCurrentTarget 0))

(event EventBeginPlay
  (bind _returnvalue (Components|GetOwner))
  (Variables|Default|SetPlayerCamera (Actor|GetComponentbyClass _returnvalue "/Script/Engine.CameraComponent"))
  (Variables|Default|SetPlayerCameraBoom (Actor|GetComponentbyClass _returnvalue "/Script/Engine.SpringArmComponent"))
  (Variables|Default|SetOwnerCharacterMovement (Actor|GetComponentbyClass _returnvalue "/Script/Engine.CharacterMovementComponent")))

(event EventTick
  (params (DeltaSeconds :type Float%20%28single-precision%29))
  (Variables|Default|GetCurrentTarget
    (:then
      (bind _ownercharactermovement (Variables|Default|GetOwnerCharacterMovement)
        (:then
          (Variables|/Script/Engine.CharacterMovementComponent|SetbOrientRotationToMovement _ownercharactermovement false)
          (Variables|/Script/Engine.CharacterMovementComponent|SetbUseControllerDesiredRotation _ownercharactermovement false)
          (bind _playercameraboom (Variables|Default|GetPlayerCameraBoom)
            (:then
              (Variables|/Script/Engine.SpringArmComponent|SetSocketOffset _playercameraboom (Math|Interpolation|VInterpTo (Variables|/Script/Engine.SpringArmComponent|GetSocketOffset _playercameraboom) "0, 0, 0" (Utilities|Time|GetWorldDeltaSeconds) 0.0)))
            (:else
              _))
          (bind _ascharacter (Utilities|Casting|CastToCharacter (Components|GetOwner)))
          (Pawn|SetControlRotation (Pawn|GetController _ascharacter) (Math|Rotator|FindLookatRotation (Transformation|GetWorldLocation (Variables|Default|GetPlayerCamera)) (Transformation|GetActorLocation (Variables|Default|GetCurrentTarget)))))
        (:else)))
    (:else
      (bind _ownercharactermovement_2 (Variables|Default|GetOwnerCharacterMovement)
        (:then
          (Variables|/Script/Engine.CharacterMovementComponent|SetbOrientRotationToMovement _ownercharactermovement_2 true)
          (Variables|/Script/Engine.CharacterMovementComponent|SetbUseControllerDesiredRotation _ownercharactermovement_2 true)
          (bind _playercameraboom_2 (Variables|Default|GetPlayerCameraBoom)
            (:then
              (Variables|/Script/Engine.SpringArmComponent|SetSocketOffset _playercameraboom_2 (Math|Interpolation|VInterpTo (Variables|/Script/Engine.SpringArmComponent|GetSocketOffset _playercameraboom_2) "0, 0, 0" (Utilities|Time|GetWorldDeltaSeconds) 0.0)))
            (:else)))
        (:else)))))

(fn FindTarget
  (params (Potential%20Targets :type Array%20of%20Actor%20Object%20References))
  (bind _returnvalue (Components|GetOwner))
  (bind _returnvalue_2 (Transformation|GetActorLocation _returnvalue))
  (bind (_outhits _returnvalue_3) (Collision|MultiSphereTraceForObjects _returnvalue_2 (+ _returnvalue_2 (* (Math|Vector|GetForwardVector (Variables|Default|GetPlayerCamera)) 1e+03)) 5e+02 (Utilities|Array|MakeArray "ObjectTypeQuery3") false (Utilities|Array|MakeArray _returnvalue) "ForDuration"))
  (if _returnvalue_3
    (Development|PrintString (Utilities|String|ToString(Integer) (Utilities|Array|Length _outhits)))))

(fn Targeting
  (bind (_return_value _found_target) (CallFunction|FindTarget (Variables|Default|GetL%20Potential%20Targets)))
  (if _return_value
    (Utilities|Array|Add (Variables|Default|GetL%20Dots) (Math|Vector|DotProduct (Math|Vector|Normalize (- (Transformation|GetActorLocation _found_target) (Transformation|GetActorLocation (Components|GetOwner)))) (Math|Vector|GetForwardVector (Variables|Default|GetPlayerCamera))))
    (else
      (return (Utilities|IsValid (Utilities|Array|Get(acopy) (Utilities|Array|MakeArray _found_target) (.IndexOfMaxValue (Math|Float|MaxOfFloatArray (Variables|Default|GetL%20Dots))))) (Utilities|Array|Get(acopy) (Utilities|Array|MakeArray _found_target) (.IndexOfMaxValue (Math|Float|MaxOfFloatArray (Variables|Default|GetL%20Dots))))))))

(fn FaceTargetDirection
  (bind _returnvalue (Components|GetOwner))
  (Transformation|SetActorRotation _returnvalue (Math|Rotator|MakeRotator 0.0 0.0 (.yaw (Math|Rotator|FindLookatRotation (Transformation|GetActorLocation _returnvalue) (Transformation|GetActorLocation (Variables|Default|GetCurrentTarget)))))))